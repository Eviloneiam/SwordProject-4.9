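; Procedural building facade that tiles modular meshes from the actor toward EndPoint in the construction script.
; EndPoint's horizontal length sets the column count and its height sets the floor count, both stepped by MeshWidth.
; MeshToSpawn forms the ground row and MeshToSpawn02 the upper floors, each tile its own InstancedStaticMesh component rather than an added instance.
; The actor's yaw turns to face EndPoint.
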(event EventBeginPlay)

(event EventActorBeginOverlap
  (params (OtherActor :type Actor%20Object%20Reference)))

(event EventTick
  (params (DeltaSeconds :type Float%20%28single-precision%29)))

(fn ConstructionScript
  (bind _returnvalue (Transformation|GetActorLocation))
  (bind _returnvalue_2 (Transformation|GetActorLocation))
  (bind _endpoint (Variables|Default|GetEndPoint))
  (bind _meshwidth (Variables|Default|GetMeshWidth))
  (bind _meshwidth_2 (Variables|Default|GetMeshWidth))
  (bind _meshtospawn_02 (Variables|Default|GetMeshToSpawn_02))
  (bind _returnvalue_3 (* _endpoint "1.000000,1.000000,0.000000"))
  (bind _returnvalue_4 (* _endpoint "0, 0,1.000000"))
  (bind _returnvalue_5 (Math|Vector|VectorLength _returnvalue_4))
  (bind _returnvalue_6 (Math|Vector|VectorLength _returnvalue_3))
  (bind _returnvalue_7 (/ _returnvalue_5 _meshwidth))
  (bind _returnvalue_8 (/ _returnvalue_6 _meshwidth_2))
  (bind _returnvalue_9 (Math|Float|Round _returnvalue_7))
  (bind _returnvalue_10 (Math|Float|Round _returnvalue_8))
  (bind _returnvalue_11 (- _returnvalue_9 1))
  (bind _returnvalue_12 (- _returnvalue_10 1))
  (Components|StaticMesh|SetStaticMesh (Variables|Default|GetBuilding_Start) (Variables|Default|GetMeshToSpawn))
  (Utilities|FlowControl|Sequence
    (:then_0
      (if (> _returnvalue_12 1)
        (for _index (range 1 _returnvalue_12)
          (bind _returnvalue_13 (AddComponent|AddInstancedStaticMeshComponent true))
          (Class|SceneComponent|Attachto _returnvalue_13 (Variables|Default|GetBuilding_Start) "None" "KeepWorldPosition" true)
          (Transformation|SetRelativeLocation _returnvalue_13 (Math|Vector|MakeVector (* _index (Variables|Default|GetMeshWidth)) 0.0 0.0) false)
          (Components|StaticMesh|SetStaticMesh _returnvalue_13 (Variables|Default|GetMeshToSpawn))))
      (Transformation|SetWorldRotation (Class|KismetMathLibrary|MakeRot 0.0 (.Yaw (Class|KismetMathLibrary|BreakRot (Math|Rotator|FindLookatRotation _returnvalue (+ _returnvalue (Variables|Default|GetEndPoint))))) 0.0) false))
    (:then_1
      (if (> _returnvalue_11 1)
        (for _index_2 (range 1 _returnvalue_11)
          (bind _returnvalue_14 (AddComponent|AddInstancedStaticMeshComponent true))
          (Class|SceneComponent|Attachto _returnvalue_14 (Variables|Default|GetBuilding_Start) "None" "KeepWorldPosition" true)
          (Transformation|SetRelativeLocation _returnvalue_14 (Math|Vector|MakeVector 0.0 0.0 (* _index_2 (Variables|Default|GetMeshWidth))) false)
          (Components|StaticMesh|SetStaticMesh _returnvalue_14 _meshtospawn_02)
          (for _index_3 (range 1 _returnvalue_12)
            (bind _returnvalue_15 (AddComponent|AddInstancedStaticMeshComponent true))
            (Class|SceneComponent|Attachto _returnvalue_15 (Variables|Default|GetBuilding_Start) "None" "KeepWorldPosition" true)
            (Transformation|SetRelativeLocation _returnvalue_15 (+ (Math|Vector|MakeVector (* _index_3 (Variables|Default|GetMeshWidth)) 0.0 0.0) (Math|Vector|MakeVector 0.0 0.0 (* _index_2 (Variables|Default|GetMeshWidth)))) false)
            (Components|StaticMesh|SetStaticMesh _returnvalue_15 _meshtospawn_02)
            (for _index_4 (range 1 0)
              _))
          (|CollapseGraph_0)))
      (Transformation|SetWorldRotation (Class|KismetMathLibrary|MakeRot 0.0 (.Yaw (Class|KismetMathLibrary|BreakRot (Math|Rotator|FindLookatRotation _returnvalue_2 (+ _returnvalue_2 (Variables|Default|GetEndPoint))))) 0.0) false))))