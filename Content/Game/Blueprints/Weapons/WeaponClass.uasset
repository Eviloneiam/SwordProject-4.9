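; Weapon actor that provides a hitscan shot through its Shoot12 event.
; The event prints a debug message, then line-traces by object type from the actor's own location along player 0's control rotation, with debug drawing on.
; On a hit it applies the Damage variable to the hit actor.
; The other events and the construction script are empty.
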(event EventShoot12
  (bind _returnvalue (Transformation|GetActorLocation))
  (Development|PrintString "Hello")
  (bind (_outhit _returnvalue_2) (Collision|LineTraceForObjects _returnvalue (+ _returnvalue (* (Math|Vector|GetForwardVector (Pawn|GetControlRotation (Game|GetPlayerController 0) :!class /Script/Engine.Controller)) 1e+04)) (Utilities|Array|MakeArray "ObjectTypeQuery1" "ObjectTypeQuery8" "ObjectTypeQuery2") false 0 "ForDuration"))
  (if _returnvalue_2
    (Game|Damage|ApplyDamage (.HitActor (Collision|BreakHitResult _outhit)) (Variables|Default|GetDamage) 0 0)))

(event EventBeginPlay)

(event EventActorBeginOverlap
  (params (OtherActor :type Actor%20Object%20Reference)))

(event EventTick
  (params (DeltaSeconds :type Float%20%28single-precision%29)))

(fn ConstructionScript)